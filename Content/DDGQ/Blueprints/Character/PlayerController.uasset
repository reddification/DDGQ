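; Player controller that owns the player's lives, collectible count and HUD, taking its limits from the DDGQ game mode's rules.
; It binds the main character's events to update the HUD, and wraps collectibles at the maximum to award a life and refill HP.
; On death it decrements lives, unpossesses and broadcasts Died; on respawn it destroys the old pawn, possesses and rebinds the new one.
; Pausing hides the HUD and broadcasts a pause request.
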(event Custom|On%20invincibility%20time%20changed
  (params (Progress :type Float%20%28single-precision%29))
  (Default|UpdateInvincibilityTimer (Variables|Default|GetHUD) Progress))

(event Custom|On%20Respawned
  (params (Character :type Main%20Character%20Object%20Reference))
  (Actor|DestroyActor (Variables|Default|GetPlayerCharacter))
  (Pawn|Possess Character)
  (CallFunction|SetUpCharacter Character)
  (HUD|RefreshHUD))

(event Custom|On%20invincibility%20state%20changed
  (params (IsInvincible :type Boolean))
  (Default|UpdateInvincibilityControlVisibility (Variables|Default|GetHUD) IsInvincible))

(event Custom|On%20Hp%20Changed
  (params (HP :type Integer))
  (Default|UpdateHP (Variables|Default|GetHUD) HP))

(event EventBeginPlay
  (Utilities|FlowControl|Sequence
    (:then_0
      (bind _asmain_character (Utilities|Casting|CastToMainCharacter (Game|GetPlayerCharacter 0)))
      (CallFunction|SetUpCharacter _asmain_character))
    (:then_1
      (HUD|SetUpHUD))
    (:then_2
      (HUD|RefreshHUD))))

(event Input|ActionEvents|InputActionPause
  (params (Key :type Key%20Structure))
  (:Pressed
    (HUD|SetHUDVisibility false)
    (Default|CallPauseRequested)))

(fn ConstructionScript
  (bind _asddgqgame_mode (Utilities|Casting|CastToDDGQGameMode (Game|GetGameMode)))
  (bind _rules (Default|GetRules _asddgqgame_mode))
  (Variables|Default|SetGameRules _rules))

(fn Die
  (bind _result (Math|Integer|DecrementInt (Variables|Default|GetLives))
    (:%20%20
      (Default|UpdateLivesCount (Variables|Default|GetHUD) _result)
      (Pawn|UnPossess)
      (Default|CallDied _result)
      (return))))

(fn PickUpCollectible
  (params (Points :type Byte))
  (Utilities|FlowControl|Sequence
    (:then_0
      (bind _output_get (LocalVariables|SetTotalCollectibles (+ (Variables|Default|GetCollectibles) Points)))
      (Variables|Default|SetCollectibles (Class|KismetMathLibrary|PercentByteByte _output_get (.MaxCollectibles (Utilities|Struct|BreakGameRules (Variables|Default|GetGameRules))))))
    (:then_1
      (Default|UpdateCollectiblesCount (Variables|Default|GetHUD) (Variables|Default|GetCollectibles)))
    (:then_2
      (if (>= (LocalVariables|GetTotalCollectibles) (.MaxCollectibles (Utilities|Struct|BreakGameRules (Variables|Default|GetGameRules))))
        (State|AddLife)))))

(fn AddLife
  (bind _gamerules (Variables|Default|GetGameRules))
  (bind _hud (Variables|Default|GetHUD))
  (bind _playercharacter (Variables|Default|GetPlayerCharacter))
  (bind (_maxcollectibles _maxlives _maxhp) (Utilities|Struct|BreakGameRules _gamerules))
  (Utilities|FlowControl|Sequence
    (:then_0
      (if (< (+ (Variables|Default|GetLives) 1) _maxlives)
        (bind _output_get (Variables|Default|SetLives (+ (Variables|Default|GetLives) 1)))
        (Default|UpdateLivesCount _hud _output_get)))
    (:then_1
      (if (< (Variables|/Game/DDGQ/Blueprints/Character/MainCharacter.MainCharacter_C|GetHitPoints _playercharacter) _maxhp)
        (bind _output_get_2 (Variables|/Game/DDGQ/Blueprints/Character/MainCharacter.MainCharacter_C|SetHitPoints _playercharacter _maxhp))
        (Default|UpdateHP _hud _output_get_2)))))

(fn SetUpHUD
  (bind _returnvalue (UserInterface|CreateWidget "/Game/DDGQ/HUD/HUD.HUD_C" self))
  (bind _output_get (Variables|Default|SetHUD _returnvalue))
  (UserInterface|Viewport|AddtoViewport _output_get 0))

(fn RefreshHUD
  (bind _hud (Variables|Default|GetHUD))
  (Default|UpdateLivesCount _hud (Variables|Default|GetLives))
  (Default|UpdateCollectiblesCount _hud (Variables|Default|GetCollectibles))
  (Default|UpdateHP _hud (Variables|/Game/DDGQ/Blueprints/Character/MainCharacter.MainCharacter_C|GetHitPoints (Variables|Default|GetPlayerCharacter)))
  (Default|UpdateInvincibilityControlVisibility _hud false))

(fn SetUpCharacter
  (params (Character :type Main%20Character%20Object%20Reference))
  (Utilities|FlowControl|Sequence
    (:then_0
      (bind _output_get (Variables|Default|SetPlayerCharacter Character)))
    (:then_1
      (EventDispatchers|BindEventtoPickedUpCollectible _output_get (EventDispatchers|CreateEvent :!event PickUpCollectible))
      (EventDispatchers|BindEventtoDied _output_get (EventDispatchers|CreateEvent :!event Die))
      (EventDispatchers|BindEventtoHpChanged _output_get (EventDispatchers|CreateEvent :!event Custom|On%20Hp%20Changed))
      (EventDispatchers|BindEventtoInvincibilityStateChanged _output_get (EventDispatchers|CreateEvent :!event Custom|On%20invincibility%20state%20changed))
      (EventDispatchers|BindEventtoInvincibilityTimeChanged _output_get (EventDispatchers|CreateEvent :!event Custom|On%20invincibility%20time%20changed))
      (EventDispatchers|BindEventtoPickedUpNewLife _output_get (EventDispatchers|CreateEvent :!event AddLife)))))

(fn SetHUDVisibility
  (params (Is%20Visible :type Boolean))
  (bind _hud (Variables|Default|GetHUD))
  (Utilities|IsValid _hud
    (:Is%20Valid
      (if Is%20Visible
        (UserInterface|Viewport|AddtoViewport _hud 0)
        (else
          (Widget|RemovefromParent _hud))))))