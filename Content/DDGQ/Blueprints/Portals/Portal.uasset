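; Portal actor that sends the MainCharacter to the level named by its LevelName variable.
; On BeginPlay it creates a PortalInfo widget carrying that level name.
; The Box trigger adds the widget to the viewport on overlap and removes it on exit.
; Overlapping Collision fires the OnLevelLoading dispatcher, then opens the level by name.
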(event OnComponentBeginOverlap(Collision)
  (params (OverlappedComponent :type Primitive%20Component%20Object%20Reference) (OtherActor :type Actor%20Object%20Reference) (OtherComp :type Primitive%20Component%20Object%20Reference) (OtherBodyIndex :type Integer) (bFromSweep :type Boolean) (SweepResult :type Hit%20Result%20Structure%20%28by%20ref%29))
  (Utilities|Casting|CastToMainCharacter OtherActor)
  (Default|CallOnLevelLoading)
  (Game|OpenLevel(byName) (Variables|Default|GetLevelName)))

(event OnComponentBeginOverlap(Box)
  (params (OverlappedComponent :type Primitive%20Component%20Object%20Reference) (OtherActor :type Actor%20Object%20Reference) (OtherComp :type Primitive%20Component%20Object%20Reference) (OtherBodyIndex :type Integer) (bFromSweep :type Boolean) (SweepResult :type Hit%20Result%20Structure%20%28by%20ref%29))
  (Utilities|Casting|CastToMainCharacter OtherActor)
  (UserInterface|Viewport|AddtoViewport (Variables|Default|GetPortalInfoWidget) 0))

(event OnComponentEndOverlap(Box)
  (params (OverlappedComponent :type Primitive%20Component%20Object%20Reference) (OtherActor :type Actor%20Object%20Reference) (OtherComp :type Primitive%20Component%20Object%20Reference) (OtherBodyIndex :type Integer))
  (bind _portalinfowidget (Variables|Default|GetPortalInfoWidget))
  (Utilities|Casting|CastToMainCharacter OtherActor)
  (Utilities|IsValid _portalinfowidget
    (:Is%20Valid
      (Widget|RemovefromParent _portalinfowidget))))

(event EventBeginPlay
  (bind _returnvalue (UserInterface|CreateWidget "/Game/DDGQ/Blueprints/Portals/PortalInfo.PortalInfo_C" 0 (Utilities|Text|ToText(Name) (Variables|Default|GetLevelName))))
  (Variables|Default|SetPortalInfoWidget _returnvalue))

(fn ConstructionScript)