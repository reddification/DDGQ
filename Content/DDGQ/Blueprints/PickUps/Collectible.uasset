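; Collectible pickup actor that comes in Small, Middle and Large types, each with its own color, point value and scale.
; The construction script looks up the type's data to tint the mesh material, store points and color, and scale the mesh.
; When the third-person character overlaps the collision, a timeline lerps the actor toward the player, then notifies the character of the pickup and destroys itself.
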(event OnComponentBeginOverlap(Collision)
  (params (OverlappedComponent :type Primitive%20Component%20Object%20Reference) (OtherActor :type Actor%20Object%20Reference) (OtherComp :type Primitive%20Component%20Object%20Reference) (OtherBodyIndex :type Integer) (bFromSweep :type Boolean) (SweepResult :type Hit%20Result%20Structure%20%28by%20ref%29))
  (bind _asthird_person_character (Utilities|Casting|CastToThirdPersonCharacter OtherActor))
  (bind _distance (Timeline|Attraction Play)
    (:Update
      (Transformation|SetActorLocation (Math|Vector|Lerp(Vector) (Transformation|GetActorLocation) (Transformation|GetActorLocation _asthird_person_character) _distance) false false))
    (:Finished
      (Default|PickedUpCollectible _asthird_person_character self)
      (Actor|DestroyActor))))

(event EventBeginPlay)

(event Collision|EventActorBeginOverlap
  (params (OtherActor :type Actor%20Object%20Reference)))

(event EventTick
  (params (DeltaSeconds :type Float%20%28single-precision%29)))

(fn ConstructionScript
  (bind _mesh (Variables|Default|GetMesh))
  (bind _returnvalue (Transformation|GetWorldScale _mesh))
  (bind (_x _y _z) (Math|Vector|BreakVector _returnvalue))
  (bind _collectibledata (CallFunction|GetCollectibleData (Variables|Default|GetCollectibleType)))
  (Rendering|Material|SetVectorParameterValueonMaterials (Variables|Default|GetMesh) "Color" (Math|Conversions|ToVector(LinearColor) (.Color (Utilities|Struct|BreakCollectibleData _collectibledata))))
  (Variables|Default|SetPoints (.Points (Utilities|Struct|BreakCollectibleData _collectibledata)))
  ;[1 1 1] Perhaps could be useful for particles
  (Variables|Default|SetColor (.Color (Utilities|Struct|BreakCollectibleData _collectibledata)))
  (Transformation|SetWorldScale3D (Variables|Default|GetMesh) (Math|Vector|MakeVector (* _x (.Scalemultiplier (Utilities|Struct|BreakCollectibleData _collectibledata))) (* _y (.Scalemultiplier (Utilities|Struct|BreakCollectibleData _collectibledata))) (* _z (.Scalemultiplier (Utilities|Struct|BreakCollectibleData _collectibledata))))))

(fn GetCollectibleData
  (params (collectibleType :type CollectibleType%20Enum :default "NewEnumerator0"))
  (switch Utilities|FlowControl|Switch|SwitchonCollectibleType collectibleType
    (:NewEnumerator0
      (return (Utilities|Struct|MakeCollectibleData "(R=0.802083,G=0.733449,B=0.000000,A=0.000000)" 1 0.75)))
    (:NewEnumerator1
      (return (Utilities|Struct|MakeCollectibleData "(R=0.027174,G=0.300234,B=0.666667,A=0.000000)" 5 1.0)))
    (:NewEnumerator2
      (return (Utilities|Struct|MakeCollectibleData "(R=0.875000,G=0.029829,B=0.000000,A=0.000000)" 10 1.25)))))