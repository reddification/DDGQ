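; PowerUp is a pickup actor that flies to the player and grants a power-up when touched.
; When a MainCharacter overlaps the capsule, it records a BaseRespawnInfo with its transform and PowerUp type, then a timeline lerps it toward the character.
; On finish it calls PickedUpPowerUp on the character, broadcasts the respawn info through CallOnRespawnableDestroyed, and destroys itself.
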(event OnComponentBeginOverlap(Capsule)
  (params (OverlappedComponent :type Primitive%20Component%20Object%20Reference) (OtherActor :type Actor%20Object%20Reference) (OtherComp :type Primitive%20Component%20Object%20Reference) (OtherBodyIndex :type Integer) (bFromSweep :type Boolean) (SweepResult :type Hit%20Result%20Structure%20%28by%20ref%29))
  ;[1 1 1] TODO: base class for this shit
  (bind _asmain_character (Utilities|Casting|CastToMainCharacter OtherActor))
  (bind _respawninfo (CallFunction|GetRespawnInfo))
  (bind _distance (Timeline|Timeline_0 Play)
    (:Update
      (Transformation|SetActorLocation (Math|Vector|Lerp(Vector) (Transformation|GetActorLocation) (Transformation|GetActorLocation _asmain_character) _distance) false false))
    (:Finished
      (Default|PickedUpPowerUp _asmain_character)
      (Default|CallOnRespawnableDestroyed _respawninfo)
      (Actor|DestroyActor))))

(event EventBeginPlay)

(event Collision|EventActorBeginOverlap
  (params (OtherActor :type Actor%20Object%20Reference)))

(event EventTick
  (params (DeltaSeconds :type Float%20%28single-precision%29)))

(fn ConstructionScript)

(fn GetRespawnInfo
  (bind _returnvalue (Game|ConstructObjectfromClass "/Game/DDGQ/Blueprints/Respawn/BaseRespawnInfo.BaseRespawnInfo_C" self (Transformation|GetWorldTransform (Variables|Default|GetScene)) "PowerUp_C"))
  (return _returnvalue))