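; Base environmental damage pad that hurts any actor entering its box.
; On box begin overlap, it applies its Damage value to that actor using its DamageType.
; The construction script tints the static mesh through the "Color" material parameter, setting yellow when DamageType casts to Electricity_DT.
; Three alternative color branches exist but are unconnected, so other damage types get no tint here.
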(event OnComponentBeginOverlap(Box)
  (params (OverlappedComponent :type Primitive%20Component%20Object%20Reference) (OtherActor :type Actor%20Object%20Reference) (OtherComp :type Primitive%20Component%20Object%20Reference) (OtherBodyIndex :type Integer) (bFromSweep :type Boolean) (SweepResult :type Hit%20Result%20Structure%20%28by%20ref%29))
  (Game|Damage|ApplyDamage OtherActor (Math|Conversions|ToFloat(Integer) (Variables|Default|GetDamage)) 0 0 (Variables|Default|GetDamageType)))

(event EventBeginPlay)

(event Collision|EventActorBeginOverlap
  (params (OtherActor :type Actor%20Object%20Reference)))

(event EventTick
  (params (DeltaSeconds :type Float%20%28single-precision%29)))

(fn ConstructionScript
  (Utilities|Casting|CastToElectricity_DTClass (Variables|Default|GetDamageType))
  (LocalVariables|SetPadColor (Math|Conversions|ToVector(LinearColor) "(R=0.708333,G=0.614809,B=0.014600,A=1.000000)"))
  (Rendering|Material|SetVectorParameterValueonMaterials (Variables|Default|GetStaticMesh) "Color" (LocalVariables|GetPadColor)))