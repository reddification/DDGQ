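; Base actor component for environment objects that react when the main character lands on top of them.
; On BeginPlay it binds to the owner's static mesh hit event, or deactivates itself if no mesh exists.
; A hit counts as a landing when the character is not falling, has vertical velocity, and the impact normal's angle from up is within range.
; Landings call OnLanded, an empty hook here.
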(event Custom|On%20hit
  (params (HitComponent :type Primitive%20Component%20Object%20Reference) (OtherActor :type Actor%20Object%20Reference) (OtherComp :type Primitive%20Component%20Object%20Reference) (NormalImpulse :type Vector) (Hit :type Hit%20Result%20Structure%20%28by%20ref%29))
  (bind _asmain_character (Utilities|Casting|CastToMainCharacter OtherActor))
  (bind _islandedontop (CallFunction|IsLandedonTop _asmain_character Hit))
  (if _islandedontop
    (CallFunction|OnLanded _asmain_character)))

(event EventBeginPlay
  (bind _output_get (Variables|Default|SetOwner (Components|GetOwner)))
  (Utilities|IsValid (Actor|GetComponentbyClass _output_get "/Script/Engine.StaticMeshComponent")
    (:Is%20Valid
      (Collision|BindEventtoOnComponentHit (Actor|GetComponentbyClass _output_get "/Script/Engine.StaticMeshComponent") (delegate Custom|On%20hit)))
    (:Is%20Not%20Valid
      (Components|Activation|SetActive false false))))

(fn IsLandedonTop
  (params (Character :type Character%20Object%20Reference) (Hit :type Hit%20Result%20Structure%20%28by%20ref%29))
  (bind _charactermovement (Variables|/Script/Engine.Character|GetCharacterMovement Character))
  (bind _angle (CallFunction|GetAngleBetweenVectors "0, 0,1.000000" (.ImpactNormal (Collision|BreakHitResult Hit))))
  (return (Math|Boolean|ANDBoolean (not (AI|Components|NavMovement|IsFalling _charactermovement)) (Math|Float|InRange(Float) _angle (LocalVariables|GetMinAngle) (LocalVariables|GetMaxAngle)) (> (Math|Float|Absolute(Float) (.z (Pawn|Components|CharacterMovement|GetLastUpdateVelocity _charactermovement))) 1.0))))

(fn OnLanded
  (params (Character :type Main%20Character%20Object%20Reference)))