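; A checkpoint actor, shown with an old PC screen material, that activates once when a BP_Character overlaps its box.
; Activation calls OnReached with an upright transform raised above the box's location.
; SetState, also run from the construction script, switches screen material, mesh tilt, text visibility and overlap events to match IsActivated.
; An unconnected save-game loading branch, noted as optional for reusable checkpoints, never runs.
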(event OnComponentBeginOverlap(Box)
  (params (OverlappedComponent :type Primitive%20Component%20Object%20Reference) (OtherActor :type Actor%20Object%20Reference) (OtherComp :type Primitive%20Component%20Object%20Reference) (OtherBodyIndex :type Integer) (bFromSweep :type Boolean) (SweepResult :type Hit%20Result%20Structure%20%28by%20ref%29))
  (Utilities|Casting|CastToBP_Character OtherActor)
  (if (not (Variables|Default|GetIsActivated))
    (bind _output_get (Variables|Default|SetIsActivated true))
    (CallFunction|SetState _output_get)
    (Default|CallOnReached (Math|Transform|MakeTransform (+ (.location (Transformation|GetWorldTransform (Variables|Default|GetBox))) "0, 0,200.000000")))))

(event EventBeginPlay)

(event Collision|EventActorBeginOverlap
  (params (OtherActor :type Actor%20Object%20Reference)))

(event EventTick
  (params (DeltaSeconds :type Float%20%28single-precision%29)))

(fn ConstructionScript
  (CallFunction|SetState (Variables|Default|GetIsActivated)))

(fn SetState
  (params (IsOn :type Boolean))
  (bind _checkpoint_text (Variables|Default|GetCheckpoint%20text))
  (bind _staticmesh (Variables|Default|GetStaticMesh))
  (bind _box (Variables|Default|GetBox))
  (if IsOn
    (Rendering|Material|SetMaterial _staticmesh 2 "/Game/DDGQ/Props/OldPc/M_OldPc_ScreenOn.M_OldPc_ScreenOn")
    (Transformation|SetRelativeRotation _staticmesh "0, 0,-20.000000" false false)
    (Rendering|SetVisibility _checkpoint_text false false)
    (Variables|/Script/Engine.PrimitiveComponent|SetbGenerateOverlapEvents _box false)
    (else
      (Rendering|Material|SetMaterial _staticmesh 2 "/Game/DDGQ/Props/OldPc/M_OldPc_ScreenOff.M_OldPc_ScreenOff")
      (Transformation|SetRelativeRotation _staticmesh "0, 0,20.000000" false false)
      (Rendering|SetVisibility _checkpoint_text true false)
      (Variables|/Script/Engine.PrimitiveComponent|SetbGenerateOverlapEvents _box true))))