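; Checkpoint manager that tracks the player's last checkpoint position and collects respawn info from destroyed respawnables.
; On BeginPlay it binds to every BP_Checkpoint and BaseRespawnable in the level and seeds the position slightly above the player's start.
; Event dispatchers update the stored position and fill the Respawnables list, which ClearRespawnables empties; respawning itself is not done here.
; An interface-based gathering path remains unconnected.
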(event Custom|OnCheckpointReached
  (params (CheckpointLocation :type Transform))
  (Variables|Default|SetLastCheckpointPosition (.location CheckpointLocation)))

(event Custom|On%20Respawnable%20Destroyed
  (params (RespawnInfo :type Base%20Respawn%20Info%20Object%20Reference))
  (Utilities|Array|Add (Variables|Default|GetRespawnables) RespawnInfo))

(event EventBeginPlay
  (Utilities|FlowControl|Sequence
    (:then_0
      (bind _outactors (Actor|GetAllActorsOfClass "/Game/DDGQ/Blueprints/Checkpoint/BP_Checkpoint.BP_Checkpoint_C"))
      (for _array_element _outactors
        (EventDispatchers|BindEventtoOnReached _array_element (delegate Custom|OnCheckpointReached))))
    (:then_1
      (bind _outactors_2 (Actor|GetAllActorsOfClass "/Game/DDGQ/Blueprints/Respawn/BaseRespawnable.BaseRespawnable_C"))
      (for _array_element_2 _outactors_2
        (CallFunction|SetUpRespawnable _array_element_2)))
    (:then_2
      (Variables|Default|SetLastCheckpointPosition (+ (Transformation|GetActorLocation (Game|GetPlayerCharacter 0)) "0, 0,200.000000")))))

(fn ConstructionScript)

(fn ClearRespawnables
  (Utilities|Array|Clear (Variables|Default|GetRespawnables)))

(fn SetUpRespawnable
  (params (Respawnable :type Base%20Respawnable%20Object%20Reference))
  (EventDispatchers|BindEventtoOnRespawnableDestroyed Respawnable (EventDispatchers|CreateEvent :!event Custom|On%20Respawnable%20Destroyed)))