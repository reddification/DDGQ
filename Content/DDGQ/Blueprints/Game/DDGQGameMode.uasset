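; Game mode that handles player death and checkpoint respawning.
; On BeginPlay it caches the player controller, camera manager and checkpoint manager, then binds to the controller's Died event.
; With lives left, it fades out, respawns the checkpoint manager's recorded respawnables (collectibles keep their type), spawns a new character at the last checkpoint and fades back in.
; With none left, it shows a death screen, then restarts the game.
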(event Custom|OnCharacterDied
  (params (LivesLeft :type Integer))
  (bind _checkpointmanager (Variables|Default|GetCheckpointManager))
  (bind _cameramanager (Variables|Default|GetCameraManager))
  (if (<= LivesLeft 0)
    (CameraFades|StartCameraFade _cameramanager 0.0 1.0 1.0 "(R=0.000000,G=0.000000,B=0.000000,A=1.000000)" false true)
    (bind _returnvalue (UserInterface|CreateWidget "/Game/DDGQ/HUD/DeathScreen.DeathScreen_C" (Variables|Default|GetPlayerController)))
    (UserInterface|Viewport|AddtoViewport _returnvalue 0)
    (Utilities|FlowControl|Delay (Variables|Default|GetDeath%20screen%20delay))
    (Widget|RemovefromParent _returnvalue)
    (Class|GameMode|RestartGame)
    (else
      (Utilities|FlowControl|Sequence
        (:then_0
          (CameraFades|StartCameraFade _cameramanager 0.0 1.0 1.0 "(R=0.000000,G=0.000000,B=0.000000,A=1.000000)" false true)
          (for _array_element (Variables|/Game/DDGQ/Blueprints/Checkpoint/BP_CheckpointManager.BP_CheckpointManager_C|GetRespawnables (Variables|Default|GetCheckpointManager))
            (bind _ascollectible_respawn_info (Utilities|Casting|CastToCollectibleRespawnInfo _array_element)
              (:then
                (bind _returnvalue_2 (Game|SpawnActorfromClass "/Game/DDGQ/Blueprints/PickUps/Collectible.Collectible_C" (Variables|/Game/DDGQ/Blueprints/Respawn/BaseRespawnInfo.BaseRespawnInfo_C|GetTransform _array_element) "Undefined" 0 (Variables|/Game/DDGQ/Blueprints/Respawn/CollectibleRespawnInfo.CollectibleRespawnInfo_C|GetCollectibleType _ascollectible_respawn_info) 0))
                (bind _asbase_respawnable (Utilities|Casting|CastToBaseRespawnable _returnvalue_2))
                (Default|SetUpRespawnable _checkpointmanager _asbase_respawnable))
              (:CastFailed
                (bind _returnvalue_3 (Game|SpawnActorfromClass (Variables|/Game/DDGQ/Blueprints/Respawn/BaseRespawnInfo.BaseRespawnInfo_C|GetType _array_element) (Variables|/Game/DDGQ/Blueprints/Respawn/BaseRespawnInfo.BaseRespawnInfo_C|GetTransform _array_element) "Undefined" 0 0))
                (bind _asbase_respawnable_2 (Utilities|Casting|CastToBaseRespawnable _returnvalue_3))
                (Default|SetUpRespawnable _checkpointmanager _asbase_respawnable_2)))))
        (:then_1
          (bind _returnvalue_4 (Game|SpawnActorfromClass "/Game/DDGQ/Blueprints/Character/BP_Character.BP_Character_C" (Math|Transform|MakeTransform (Variables|/Game/DDGQ/Blueprints/Checkpoint/BP_CheckpointManager.BP_CheckpointManager_C|GetLastCheckpointPosition (Variables|Default|GetCheckpointManager)) "0, 0, 0" "1,1,1") "Undefined" 0 0))
          (Default|OnRespawned (Variables|Default|GetPlayerController) _returnvalue_4)
          (Default|ClearRespawnables (Variables|Default|GetCheckpointManager))
          (CameraFades|StartCameraFade _cameramanager 1.0 0.0 1.0 "(R=0.000000,G=0.000000,B=0.000000,A=1.000000)" false true))))))

(event EventBeginPlay
  (Utilities|FlowControl|Sequence
    (:then_0
      (bind _asbp_player_controller (Utilities|Casting|CastToBP_PlayerController (Game|GetPlayerController 0)))
      (Variables|Default|SetPlayerController _asbp_player_controller)
      (Variables|Default|SetCameraManager (Game|GetPlayerCameraManager 0)))
    (:then_1
      (bind _outactors (Actor|GetAllActorsOfClass "/Game/DDGQ/Blueprints/Checkpoint/BP_CheckpointManager.BP_CheckpointManager_C"))
      (Variables|Default|SetCheckpointManager (Utilities|Array|Get(acopy) _outactors)))
    (:then_2
      (EventDispatchers|BindEventtoDied (Variables|Default|GetPlayerController) (delegate Custom|OnCharacterDied)))))

(fn ConstructionScript)

(fn GetRules
  (return (Variables|Default|GetGameRules)))